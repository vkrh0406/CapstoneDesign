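; Behavior tree decorator for enemy AI that gates a branch on whether the attack type differs from one enum value.
; The condition check returns that comparison directly, as the chain that fetches the attack type is disconnected.
; That unused chain casts to Enemy1, requires a TestCharacter player, reads the attack type and sets the IsSuccessEnemyAttack blackboard flag when the comparison passes.
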(fn PerformConditionCheckAI
  (params (OwnerController :type AI%20Controller%20Object%20Reference) (ControlledPawn :type Pawn%20Object%20Reference))
  (return (and (Utilities|Enum|NotEqual(Enum) (Utilities|Enum|LiteralenumEnum_AttackType (stale _newparam)) "NewEnumerator8") true)))