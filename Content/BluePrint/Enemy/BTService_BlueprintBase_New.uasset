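; Behavior tree service for Enemy1 that copies enemy and player combat state into the Blackboard.
; Each tick it caches the pawn and the player actor the enemy provides, except on the first, which only caches the AI controller before the write step.
; With a valid player, it writes the enemy's attack type and TestCharacter's lock-on battle mode, attack type and avoid state.
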(event EventReceiveTickAI
  (params (OwnerController :type AI%20Controller%20Object%20Reference) (ControlledPawn :type Pawn%20Object%20Reference) (DeltaSeconds :type Float%20%28single-precision%29))
  (Utilities|IsValid (Variables|Default|GetAIController)
    (:Is%20Valid
      (bind _asenemy_1 (Utilities|Casting|CastToEnemy1 ControlledPawn))
      (bind _playeractor (Default|GetPlayerActor _asenemy_1))
      (Variables|Default|SetPlayer _playeractor)
      (Variables|Default|SetEnemy _asenemy_1))
    (:Is%20Not%20Valid
      (Variables|Default|SetAIController OwnerController)))
  (Utilities|IsValid (Variables|Default|GetPlayer)
    (:Is%20Valid
      (bind _asenemy_1_2 (Utilities|Casting|CastToEnemy1 (Variables|Default|GetEnemy)))
      (bind _newparam (Default|GetEnemyAttackType _asenemy_1_2))
      (Class|BTFunctionLibrary|SetBlackboardValueasEnum (Variables|Default|GetEnemyAttackType) (Utilities|Enum|LiteralenumEnum_AttackType _newparam))
      (bind _astest_character (Utilities|Casting|CastToTestCharacter (Variables|Default|GetPlayer)))
      (Class|BTFunctionLibrary|SetBlackboardValueasBool (Variables|Default|GetBattleMode) (Variables|/Game/BluePrint/TestCharacter.TestCharacter_C|GetBattleModeLockOn _astest_character))
      (Class|BTFunctionLibrary|SetBlackboardValueasEnum (Variables|Default|GetPlayerAttackType) (Variables|/Game/BluePrint/TestCharacter.TestCharacter_C|GetEnumAttackType _astest_character))
      (Class|BTFunctionLibrary|SetBlackboardValueasBool (Variables|Default|GetPlayeAvoid) (Variables|/Game/BluePrint/TestCharacter.TestCharacter_C|GetAvoid _astest_character)))))