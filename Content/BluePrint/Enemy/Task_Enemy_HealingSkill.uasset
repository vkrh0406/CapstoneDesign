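; Behavior tree task for an enemy healing skill that restores 30% of max HP, with no clamp.
; It plays a card-cast montage, applies the heal and HP update as the montage starts, and finishes successfully when it completes.
; Montage speed is randomized: above half HP the range is fixed, while at or below half it adds a bonus that grows as HP drops to the stored bounds.
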(event EventReceiveExecuteAI
  (params (OwnerController :type AI%20Controller%20Object%20Reference) (ControlledPawn :type Pawn%20Object%20Reference))
  (bind _output_get (Variables|Default|SetEnemy (.AsEnemy%201 (Utilities|Casting|CastToEnemy1 ControlledPawn))))
  (Variables|Default|SetPlayer (.AsTest%20Character (Utilities|Casting|CastToTestCharacter (Variables|/Game/BluePrint/Enemy/Enemy1.Enemy1_C|GetPlayer _output_get))))
  (CallFunction|SetRandomAnimSpeed (Variables|/Game/BluePrint/Enemy/Enemy1.Enemy1_C|GetHP%20Monster (Variables|Default|GetEnemy)) (Variables|/Game/BluePrint/Enemy/Enemy1.Enemy1_C|GetMaxHP (Variables|Default|GetEnemy)))
  (Animation|Montage|PlayMontage (Variables|/Script/Engine.Character|GetMesh (Variables|Default|GetEnemy)) "/Game/Animation/CardCast_Montage.CardCast_Montage" (Variables|Default|GetAnimSpeed)
    (:then
      (bind _output_get_2 (Variables|/Game/BluePrint/Enemy/Enemy1.Enemy1_C|SetHP%20Monster (Variables|Default|GetEnemy) (+ (Variables|/Game/BluePrint/Enemy/Enemy1.Enemy1_C|GetHP%20Monster (Variables|Default|GetEnemy)) (* (Variables|/Game/BluePrint/Enemy/Enemy1.Enemy1_C|GetMaxHP (Variables|Default|GetEnemy)) 0.3))))
      (Default|CallUpdateHPMonster (Variables|Default|GetEnemy) _output_get_2))
    (:OnCompleted
      (AI|BehaviorTree|FinishExecute true))))

(fn SetRandomAnimSpeed
  (params (Hp :type Float%20%28single-precision%29) (MaxHp :type Float%20%28single-precision%29))
  (bind _returnvalue (/ Hp MaxHp))
  (bind _returnvalue_2 (- 0.6 _returnvalue))
  (if (<= _returnvalue 0.5)
    (Variables|Default|SetMin (+ (Variables|Default|GetMin) _returnvalue_2))
    (Variables|Default|SetMax (+ (Variables|Default|GetMax) _returnvalue_2))
    (else
      (Variables|Default|SetMin 0.3)
      (Variables|Default|SetMax 0.7)))
  (Variables|Default|SetAnimSpeed (Math|Random|RandomFloatinRange (Variables|Default|GetMin) (Variables|Default|Getmax))))