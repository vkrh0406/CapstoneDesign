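; Behavior tree task that ends an enemy's stun window and turns super armor back on.
; It polls the blackboard in a 0.2-second Delay loop until the enemy is no longer alive, takes three or more hits, or SuperTime elapses.
; It then sets SuperArmor, resets the parry and hit counters and timer, clears IsStun on the Enemy1 Greystone anim Blueprint, and finishes successfully.
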(event EventReceiveExecuteAI
  (params (OwnerController :type AI%20Controller%20Object%20Reference) (ControlledPawn :type Pawn%20Object%20Reference))
  (if (or (not (Class|BTFunctionLibrary|GetBlackboardValueasBool (Variables|Default|GetIsAlive))) (>= (Class|BTFunctionLibrary|GetBlackboardValueasInt (Variables|Default|GetHitCount)) 3)) :!label _label
    _
    (else
      (bind _output_get (Variables|Default|SetTimeNow (+ (Variables|Default|GetTimeNow) 0.2)))
      (Utilities|FlowControl|Delay 0.2)
      (if (>= _output_get (Variables|Default|GetSuperTime))
        _
        (else
          (goto _label)))))
  (Class|BTFunctionLibrary|SetBlackboardValueasBool (Variables|Default|GetSuperArmor) true)
  (Class|BTFunctionLibrary|SetBlackboardValueasInt (Variables|Default|GetParringCount))
  (Class|BTFunctionLibrary|SetBlackboardValueasInt (Variables|Default|GetHitCount))
  (Variables|Default|SetTimeNow 0.0)
  (Variables|/Game/BluePrint/Enemy/Greystone_AnimBlueprint.Greystone_AnimBlueprint_C|SetIsStun (.AsGreystone%20Anim%20Blueprint (Utilities|Casting|CastToGreystone_AnimBlueprint (Components|SkeletalMesh|GetAnimInstance (Variables|/Script/Engine.Character|GetMesh (.AsEnemy%201 (Utilities|Casting|CastToEnemy1 ControlledPawn)))))) false)
  (AI|BehaviorTree|FinishExecute true))