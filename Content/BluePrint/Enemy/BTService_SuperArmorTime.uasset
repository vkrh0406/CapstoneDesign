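; Behavior tree service for enemy AI that runs a three-second super armor timer by setting the HitCount blackboard key.
; Each AI tick adds DeltaSeconds to TimeNow, which a DoOnce zeroes on the first tick only.
; Once three seconds have accumulated, it writes 3 to HitCount on every tick, which the author's note describes as releasing super armor.
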(event EventReceiveTickAI
  (params (OwnerController :type AI%20Controller%20Object%20Reference) (ControlledPawn :type Pawn%20Object%20Reference) (DeltaSeconds :type Float%20%28single-precision%29))
  ;[1 1 1] 슈퍼아머가 꺼진뒤 시작되는 서비스로 시간이 3초 지나면 Hit Count를 3으로 변경하여 슈퍼아머 해제
  (Utilities|FlowControl|Sequence
    (:then_0
      (Utilities|FlowControl|DoOnce false
        (:Completed
          (Variables|Default|SetTimeNow 0.0))))
    (:then_1
      (Variables|Default|SetTimeNow (+ DeltaSeconds (Variables|Default|GetTimeNow)))
      (if (>= (Variables|Default|GetTimeNow) 3.0)
        (Class|BTFunctionLibrary|SetBlackboardValueasInt (Variables|Default|GetHitCount) 3)))))