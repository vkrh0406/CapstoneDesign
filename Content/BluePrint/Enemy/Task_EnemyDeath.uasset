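; Behavior tree task that runs an Enemy1's death: it starts the death montage at a negative play rate, then waits briefly.
; It clears the player's lock-on and movement-lock flags, refreshes overlaps and disables the enemy-finder collision.
; It then destroys the sword collision and enemy, spawns a blast effect, awards player EXP and finishes as failed.
; Both the montage's immediate and completed outputs feed the same delayed cleanup chain.
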(event EventReceiveExecuteAI
  (params (OwnerController :type AI%20Controller%20Object%20Reference) (ControlledPawn :type Pawn%20Object%20Reference))
  (bind _returnvalue (Game|Player|GetPlayerPawn 0))
  (bind _astest_character (Utilities|Casting|CastToTestCharacter _returnvalue))
  (bind _output_get (Variables|Default|SetEnemy (.AsEnemy%201 (Utilities|Casting|CastToEnemy1 ControlledPawn))))
  (Variables|Default|SetEnemyLocation (Transformation|GetWorldLocation (Variables|/Script/Engine.Character|GetMesh _output_get)))
  (Animation|Montage|PlayMontage (Variables|/Script/Engine.Character|GetMesh _output_get) "/Game/Animation/Death_Montage.Death_Montage" -1.0
    (:then
      _)
    (:OnCompleted
      _))
  (Utilities|FlowControl|Delay 1.0)
  (Variables|/Game/BluePrint/TestCharacter.TestCharacter_C|SetBattleModeLockOn _astest_character false)
  (Variables|/Game/BluePrint/TestCharacter.TestCharacter_C|SetNotMoveTime _astest_character false)
  (Default|Generateoverlap _astest_character)
  (Actor|DestroyActor (Variables|/Game/BluePrint/Enemy/Enemy1.Enemy1_C|GetSword_Collision (Variables|Default|GetEnemy)))
  (Collision|SetCollisionEnabled (Variables|/Game/BluePrint/TestCharacter.TestCharacter_C|GetEnemyFinderCollision _astest_character) "NoCollision")
  (Class|Pawn|DetachfromControllerPendingDestroy ControlledPawn)
  (Class|Pawn|DetachfromControllerPendingDestroy (Variables|Default|GetEnemy))
  (Actor|DestroyActor (Variables|Default|GetEnemy))
  (Effects|SpawnEmitteratLocation "/Game/InfinityBladeEffects/P_YoYo_Blast_Axe_01.P_YoYo_Blast_Axe_01" (Variables|Default|GetEnemyLocation))
  (Default|GetExp _astest_character)
  (AI|BehaviorTree|FinishExecute false))