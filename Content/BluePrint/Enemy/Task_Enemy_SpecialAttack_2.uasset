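; Behavior tree task for an enemy's second special attack, which plays the Ability_R montage and finishes when it completes.
; On the AttackTiming notify it damages the player unless they are blocking, with no range check.
; Before playing, a frozen enemy spends one of the player's SkillIce counts to slow the montage's play rate, or unfreezes when none remain.
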(event EventReceiveExecuteAI
  (params (OwnerController :type AI%20Controller%20Object%20Reference) (ControlledPawn :type Pawn%20Object%20Reference))
  (bind _output_get (Variables|Default|SetEnemy (.AsEnemy%201 (Utilities|Casting|CastToEnemy1 ControlledPawn))))
  (Variables|Default|SetPlayer (.AsTest%20Character (Utilities|Casting|CastToTestCharacter (Variables|/Game/BluePrint/Enemy/Enemy1.Enemy1_C|GetPlayer _output_get))))
  (CallFunction|SetAnimSpeedbySkill)
  (bind _notifyname (Animation|Montage|PlayMontage (Variables|/Script/Engine.Character|GetMesh (Variables|Default|GetEnemy)) "/Game/Animation/Ability_R_Montage.Ability_R_Montage" (Variables|Default|GetAnimSpeed))
    (:OnCompleted
      (AI|BehaviorTree|FinishExecute true))
    (:OnNotifyBegin
      (if (Utilities|Name|Equal(Name) _notifyname "AttackTiming") ; AttackTiming Notify 가 맞는지 확인
        (if (not (Variables|/Game/BluePrint/TestCharacter.TestCharacter_C|GetBlock (Variables|Default|GetPlayer))) ; 플레이어가 막는중인지 확인
          (Game|Damage|ApplyDamage (Variables|Default|GetPlayer) 4e+01 0 (Variables|Default|GetEnemy)) ; 막기 실패시 대미지 100
        )))))

(fn SetAnimSpeedbySkill
  (if (Variables|/Game/BluePrint/Enemy/Enemy1.Enemy1_C|GetIsFrozen (Variables|Default|GetEnemy))
    (if (>= (Variables|/Game/BluePrint/TestCharacter.TestCharacter_C|GetSkill_Ice (Variables|Default|GetPlayer)) 1)
      (Variables|Default|SetAnimSpeed (* (Variables|Default|GetAnimSpeed) 0.7))
      (Math|Integer|DecrementInt (Variables|/Game/BluePrint/TestCharacter.TestCharacter_C|GetSkill_Ice (Variables|Default|GetPlayer)))
      (else
        (Variables|/Game/BluePrint/Enemy/Enemy1.Enemy1_C|SetIsFrozen (Variables|Default|GetEnemy) false)))))