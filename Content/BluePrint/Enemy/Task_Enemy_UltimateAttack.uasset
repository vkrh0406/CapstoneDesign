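; Behavior tree task that runs the enemy's ultimate attack on the player.
; It plays the ultimate montage on the enemy's mesh and finishes successfully only when the montage completes; no interruption path is handled.
; The AttackTiming notify applies damage directly to the enemy's stored Player reference, with no range or hit check, dealing far less damage if the player is blocking.
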(event EventReceiveExecuteAI
  (params (OwnerController :type AI%20Controller%20Object%20Reference) (ControlledPawn :type Pawn%20Object%20Reference))
  (bind _output_get (Variables|Default|SetEnemy (.AsEnemy%201 (Utilities|Casting|CastToEnemy1 ControlledPawn))))
  (Variables|Default|SetPlayer (.AsTest%20Character (Utilities|Casting|CastToTestCharacter (Variables|/Game/BluePrint/Enemy/Enemy1.Enemy1_C|GetPlayer _output_get))))
  (bind _notifyname (Animation|Montage|PlayMontage (Variables|/Script/Engine.Character|GetMesh (Variables|Default|GetEnemy)) "/Game/Animation/Ability_Ultimate_Montage.Ability_Ultimate_Montage")
    (:OnCompleted
      (AI|BehaviorTree|FinishExecute true))
    (:OnNotifyBegin
      (if (Utilities|Name|Equal(Name) _notifyname "AttackTiming") ; AttackTiming Notify 가 맞는지 확인
        (if (Variables|/Game/BluePrint/TestCharacter.TestCharacter_C|GetBlock (Variables|Default|GetPlayer)) ; 플레이어가 막는중인지 확인
          (Game|Damage|ApplyDamage (Variables|Default|GetPlayer) 1e+01 0 (Variables|Default|GetEnemy)) ; 막기 성공시 대미지 10
          (else
            (Game|Damage|ApplyDamage (Variables|Default|GetPlayer) 1e+02 0 (Variables|Default|GetEnemy)) ; 막기 실패시 대미지 100
          ))))))