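; Player character with HUD, pause and inventory widgets, test keys for stats, and a lock-on swipe-combat mode.
; Overlapping an "Enemy" blocks movement, then Delay loops turn and walk the player toward it before Tick holds the lock-on.
; A/D trigger cooldown-limited timeline dodges.
; Mouse swipes spawn trail particles, classify into eight attack types, and print success by screen-space distance to the target's HitPoint.
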(event OnComponentBeginOverlap(EnemyFinderCollision)
  (params (OverlappedComponent :type Primitive%20Component%20Object%20Reference) (OtherActor :type Actor%20Object%20Reference) (OtherComp :type Primitive%20Component%20Object%20Reference) (OtherBodyIndex :type Integer) (bFromSweep :type Boolean) (SweepResult :type Hit%20Result%20Structure%20%28by%20ref%29))
  (bind _returnvalue (Pawn|GetControlRotation :!class /Script/Engine.Pawn))
  (bind _returnvalue_2 (Game|GetPlayerController 0))
  ;[1 1 1] 몬스터와 가까워지면 사용자의 입력을 막고 시선을 몬스터 앞쪽으로 천천히 옮기는 루프
  (if (Actor|ActorHasTag OtherActor "Enemy")
    (Variables|전투|SetLockonTarget OtherActor)
    (Variables|전투|SetNotMoveTime true)
    (Utilities|FlowControl|Delay 0.0 :!label _label)
    (Pawn|SetControlRotation (Game|GetPlayerController 0) (Math|Interpolation|RInterpTo _returnvalue (Math|Rotator|FindLookatRotation (Transformation|GetWorldLocation (Variables|Default|GetCamera)) (+ (Transformation|GetActorLocation (Variables|전투|GetLockonTarget)) "100.000000, 0,200.000000")) (Variables|Default|GetDeltaTime) 2.0))
    (if (Math|Rotator|Equal(Rotator) _returnvalue (Math|Rotator|FindLookatRotation (Transformation|GetWorldLocation (Variables|Default|GetCamera)) (+ (Transformation|GetActorLocation (Variables|전투|GetLockonTarget)) "100.000000, 0,200.000000")) 2.0)
      ;[1 1 1] 몬스터 앞으로 캐릭터가 이동하는 루프
      (Utilities|FlowControl|Delay 0.0 :!label _label_2)
      (Pawn|Input|AddMovementInput (Math|Vector|GetForwardVector (Variables|Default|GetCamera)) 1.0 false)
      (if (Math|Vector|Equal(Vector) (+ (Transformation|GetActorLocation (Variables|전투|GetLockonTarget)) "100.000000, 0,200.000000") (Transformation|GetWorldLocation (Variables|Default|GetCamera)) 1e+02)
        (Variables|전투|SetBattleModeLockOn true)
        (Input|SetInputModeGameandUI _returnvalue_2 0 "DoNotLock" false)
        (Variables|/Script/Engine.PlayerController|SetbShowMouseCursor _returnvalue_2 true)
        (else
          (goto _label_2)))
      (else
        (goto _label)))))

(event OnComponentEndOverlap(EnemyFinderCollision)
  (params (OverlappedComponent :type Primitive%20Component%20Object%20Reference) (OtherActor :type Actor%20Object%20Reference) (OtherComp :type Primitive%20Component%20Object%20Reference) (OtherBodyIndex :type Integer)))

(event EventBeginPlay
  (bind _returnvalue (UserInterface|CreateWidget "/Game/BluePrint/HUDWidget.HUDWidget_C"))
  (bind _output_get (Variables|Default|SetHUDRef _returnvalue))
  (UserInterface|Viewport|AddtoViewport _output_get 0)
  (Input|SetInputModeGameOnly (Game|GetPlayerController 0)))

(event Collision|EventActorBeginOverlap
  (params (OtherActor :type Actor%20Object%20Reference)))

(event EventTick
  (params (DeltaSeconds :type Float%20%28single-precision%29))
  (bind _returnvalue (Game|GetPlayerController 0))
  (bind _lockontarget (Variables|전투|GetLockonTarget))
  (bind (_hitresult _returnvalue_2) (Game|Player|GetHitResultUnderCursorbyChannel _returnvalue "TraceTypeQuery1" true))
  (bind _output_get (Variables|Default|SetDeltaTime DeltaSeconds))
  (Variables|전투|SetAvoidCoolTime (+ (Variables|전투|GetAvoidCoolTime) _output_get))
  ;[1 1 1] 캐릭터가 몬스터와 콜리전 오버랩될때의 락온기능
  (if (Variables|전투|GetBattleModeLockOn)
    (Utilities|IsValid _lockontarget
      (:Is%20Valid
        (Pawn|SetControlRotation (Game|GetPlayerController 0) (Math|Interpolation|RInterpTo (Pawn|GetControlRotation :!class /Script/Engine.Pawn) (Math|Rotator|FindLookatRotation (Transformation|GetWorldLocation (Variables|Default|GetCamera)) (+ (Transformation|GetActorLocation _lockontarget) "0, 0,200.000000")) (Variables|Default|GetDeltaTime) 5.0))
        (Variables|전투|SetBattleModeLockOn true)
        ;[1 1 1] 마우스 트레일 이펙트
        (Utilities|FlowControl|Gate true
          (:Exit
            (if _returnvalue_2
              (Effects|SpawnEmitteratLocation "/Game/StarterContent/Particles/P_Explosion.P_Explosion" (.Location (Collision|BreakHitResult _hitresult)) "0, 0, 0" "0.100000,0.100000,0.100000"))))))))

(event Input|ActionEvents|InputActionJump
  (params (Key :type Key%20Structure))
  (:Pressed
    (if (not (Variables|전투|GetNotMoveTime))
      (Character|Jump))))

(event Input|AxisEvents|InputAxisForward
  (params (AxisValue :type Float%20%28single-precision%29))
  (if (not (Variables|전투|GetNotMoveTime))
    (Pawn|Input|AddMovementInput (Math|Vector|GetForwardVector (Variables|Default|GetCamera)) AxisValue false)))

(event Input|AxisEvents|InputAxisRight
  (params (AxisValue :type Float%20%28single-precision%29))
  (if (not (Variables|전투|GetNotMoveTime))
    (Pawn|Input|AddMovementInput (Math|Vector|GetRightVector (Variables|Default|GetCamera)) AxisValue false)))

(event Input|AxisEvents|InputAxisLookUp
  (params (AxisValue :type Float%20%28single-precision%29))
  (if (not (Variables|전투|GetNotMoveTime))
    (Pawn|Input|AddControllerPitchInput AxisValue)))

(event Input|AxisEvents|InputAxisLookRight
  (params (AxisValue :type Float%20%28single-precision%29))
  (if (not (Variables|전투|GetNotMoveTime))
    (Pawn|Input|AddControllerYawInput AxisValue)))

(event Input|KeyboardEvents|J
  (params (Key :type Key%20Structure))
  ;[1 1 1] 각종 상호작용 키 (임시인것도 있음)
  (:Pressed
    (bind _output_get (Variables|Default|SetWeapon (- (Variables|Default|GetWeapon) 5.0)))
    (Default|CallUpdateWeapon _output_get)))

(event Input|KeyboardEvents|F
  (params (Key :type Key%20Structure))
  ;[1 1 1] 각종 상호작용 키 (임시인것도 있음)
  (:Pressed
    (bind _output_get (Variables|Default|SetHP (- (Variables|Default|GetHP) 1.0)))
    (Default|CallUpdateHP _output_get)))

(event Input|KeyboardEvents|I
  (params (Key :type Key%20Structure))
  (bind _returnvalue (Game|GetPlayerController 0))
  (bind _returnvalue_2 (Game|GetPlayerController 0))
  ;[1 1 1] 인벤토리
  (:Pressed
    (Utilities|FlowControl|FlipFlop
      (:A
        (bind _returnvalue_3 (UserInterface|CreateWidget "/Game/BluePrint/Inventory.Inventory_C"))
        (bind _output_get (Variables|Default|SetInventoryRef _returnvalue_3))
        (UserInterface|Viewport|AddtoViewport _output_get 0)
        (Input|SetInputModeUIOnly _returnvalue_2 _output_get "DoNotLock")
        (Variables|/Script/Engine.PlayerController|SetbShowMouseCursor _returnvalue_2 true))
      (:B
        (Widget|RemovefromParent (Variables|Default|GetInventoryRef))
        (Input|SetInputModeGameOnly _returnvalue)
        (Variables|/Script/Engine.PlayerController|SetbShowMouseCursor _returnvalue false)))))

(event Input|MouseEvents|LeftMouseButton
  (params (Key :type Key%20Structure))
  (bind _returnvalue (Game|GetPlayerController 0))
  (bind (_hitresult _returnvalue_2) (Game|Player|GetHitResultUnderCursorbyChannel _returnvalue "TraceTypeQuery1" true))
  ;[1 1 1] 마우스 트레일 이펙트
  (:Pressed
    (Utilities|FlowControl|Gate true) ; enters at Open
  )
  (:Released
    (Utilities|FlowControl|Gate true) ; enters at Close
  ))

(event Input|KeyboardEvents|G
  (params (Key :type Key%20Structure))
  ;[1 1 1] 각종 상호작용 키 (임시인것도 있음)
  (:Pressed
    (bind _output_get (Variables|Default|SetHP (- (Variables|Default|GetHP) 35.0)))
    (Default|CallUpdateHP _output_get)))

(event Input|KeyboardEvents|K
  (params (Key :type Key%20Structure))
  ;[1 1 1] 각종 상호작용 키 (임시인것도 있음)
  (:Pressed
    (bind _output_get (Variables|Default|SetShield (- (Variables|Default|GetShield) 5.0)))
    (Default|CallUpdateShield _output_get)))

(event Input|KeyboardEvents|L
  (params (Key :type Key%20Structure))
  ;[1 1 1] 각종 상호작용 키 (임시인것도 있음)
  (:Pressed
    (bind _output_get (Variables|Default|SetArmor (- (Variables|Default|GetArmor) 5.0)))
    (Default|CallUpdateArmor _output_get)))

(event Input|KeyboardEvents|1
  (params (Key :type Key%20Structure))
  (bind _max_hp (Variables|Default|GetMax%20Hp))
  ;[1 1 1] 각종 상호작용 키 (임시인것도 있음)
  ;;[1 1 1] 체력회복
  (:Pressed
    (Variables|Default|SetPressed1 true)
    (if (> (+ (Variables|Default|GetHP) 2e+01) _max_hp)
      (bind _output_get (Variables|Default|SetHP _max_hp))
      (Default|CallUpdateHP _output_get)
      (Development|PrintString (Utilities|String|ToString(Float) _output_get))
      (else
        (bind _output_get_2 (Variables|Default|SetHP (+ (Variables|Default|GetHP) 2e+01)))
        (Default|CallUpdateHP _output_get_2)
        (Development|PrintString (Utilities|String|ToString(Float) _output_get_2)))))
  (:Released
    (Variables|Default|SetPressed1 false)))

(event Input|KeyboardEvents|2
  (params (Key :type Key%20Structure))
  ;[1 1 1] 각종 상호작용 키 (임시인것도 있음)
  (:Pressed
    (Variables|Default|SetPressed2 true))
  (:Released
    (Variables|Default|SetPressed2 false)))

(event Input|KeyboardEvents|A
  (params (Key :type Key%20Structure))
  (bind _mesh (Variables|Character|GetMesh))
  (bind _camera (Variables|Default|GetCamera))
  (bind _relativelocation (Variables|/Script/Engine.SceneComponent|GetRelativeLocation _mesh))
  (bind _relativelocation_2 (Variables|/Script/Engine.SceneComponent|GetRelativeLocation _camera))
  (bind (_x _y) (Math|Vector|BreakVector _relativelocation))
  (bind (_x_2 _y_2) (Math|Vector|BreakVector _relativelocation_2))
  ;[1 1 1] A 또는 D 누르면 왼쪽 오른쪽 회피이동
  (:Pressed
    (if (Math|Boolean|ANDBoolean (Variables|전투|GetNotMoveTime) (<= 1.0 (Variables|전투|GetAvoidCoolTime)) (Variables|전투|GetBattleModeLockOn))
      (Variables|전투|SetBattleModeLockOn false)
      (Variables|전투|SetAvoidCoolTime 0.0)
      (bind (_direction _addmovement _height _cameraheight _cameraheight2) (Timeline|AvoidMovement PlayFromStart)
        (:Update
          (Pawn|Input|AddMovementInput (* (Math|Vector|GetRightVector (Variables|Default|GetCamera)) "1.000000,-1.000000,1.000000") (Math|Float|Lerp 0.0 1.0 _addmovement) false)
          (Transformation|SetRelativeLocation _camera (Math|Vector|MakeVector _x_2 _y_2 _cameraheight) false false)
          (Transformation|SetRelativeLocation _mesh (Math|Vector|MakeVector _x _y _cameraheight2) false false))
        (:Finished
          (Variables|전투|SetBattleModeLockOn true)
          (Development|PrintString "Avoid Success"))))))

(event Input|KeyboardEvents|D
  (params (Key :type Key%20Structure))
  (bind _mesh (Variables|Character|GetMesh))
  (bind _camera (Variables|Default|GetCamera))
  (bind _relativelocation (Variables|/Script/Engine.SceneComponent|GetRelativeLocation _mesh))
  (bind _relativelocation_2 (Variables|/Script/Engine.SceneComponent|GetRelativeLocation _camera))
  (bind (_x _y) (Math|Vector|BreakVector _relativelocation))
  (bind (_x_2 _y_2) (Math|Vector|BreakVector _relativelocation_2))
  ;[1 1 1] A 또는 D 누르면 왼쪽 오른쪽 회피이동
  (:Pressed
    (if (Math|Boolean|ANDBoolean (Variables|전투|GetNotMoveTime) (<= 1.0 (Variables|전투|GetAvoidCoolTime)) (Variables|전투|GetBattleModeLockOn))
      (Variables|전투|SetBattleModeLockOn false)
      (Variables|전투|SetAvoidCoolTime 0.0)
      (bind (_direction _addmovement _height _cameraheight _cameraheight2) (Timeline|AvoidMovement ReverseFromEnd)
        (:Update
          (Pawn|Input|AddMovementInput (* (Math|Vector|GetRightVector (Variables|Default|GetCamera)) "1.000000,-1.000000,1.000000") (Math|Float|Lerp 0.0 1.0 _addmovement) false)
          (Transformation|SetRelativeLocation _camera (Math|Vector|MakeVector _x_2 _y_2 _cameraheight) false false)
          (Transformation|SetRelativeLocation _mesh (Math|Vector|MakeVector _x _y _cameraheight2) false false))
        (:Finished
          (Variables|전투|SetBattleModeLockOn true)
          (Development|PrintString "Avoid Success"))))))

(event Input|KeyboardEvents|P
  (params (Key :type Key%20Structure))
  ;[1 1 1] Pause
  (:Pressed
    (CallFunction|PauseGame)))

(event Input|MouseEvents|LeftMouseButton
  (params (Key :type Key%20Structure))
  (bind _returnvalue (Game|GetPlayerController 0))
  (bind _returnvalue_2 (Game|GetPlayerController 0))
  (bind _returnvalue_3 (Game|GetPlayerController 0))
  (bind _lockontarget (Variables|전투|GetLockonTarget))
  (bind (_locationx _locationy) (Game|Player|GetMousePosition _returnvalue_2))
  (bind (_locationx_2 _locationy_2) (Game|Player|GetMousePosition _returnvalue_3))
  (bind _returnvalue_4 (Actor|GetComponentsbyTag _lockontarget "/Script/Engine.BoxComponent" "HitPoint"))
  (bind _returnvalue_5 (Math|Vector|MakeVector _locationx _locationy 0.0))
  (bind _output (Utilities|Array|Get(acopy) _returnvalue_4))
  (bind _returnvalue_6 (Transformation|GetWorldLocation _output))
  (bind _screenlocation (Class|PlayerController|ProjectWorldLocationtoScreen _returnvalue _returnvalue_6 false))
  (bind _returnvalue_7 (Math|Conversions|ToVector(Vector2D) _screenlocation))
  (:Pressed
    (Variables|전투|SetMousePositionPressed (Math|Vector|MakeVector _locationx_2 _locationy_2 0.0)))
  (:Released
    (bind _output_get (Variables|전투|SetUnitDirection (Math|Vector|GetUnitDirection(Vector) (Variables|전투|GetMousePositionPressed) _returnvalue_5)))
    (bind _output_get_2 (Variables|전투|SetEnemyLocationByViewport _returnvalue_7))
    (if (>= (+ (.X (Math|Vector|BreakVector (* (- (Variables|전투|GetMousePositionPressed) _returnvalue_5) (- (Variables|전투|GetMousePositionPressed) _returnvalue_5)))) (.Y (Math|Vector|BreakVector (* (- (Variables|전투|GetMousePositionPressed) _returnvalue_5) (- (Variables|전투|GetMousePositionPressed) _returnvalue_5))))) 5e+04)
      (if (and (and (<= (.X (Math|Vector|BreakVector (Variables|전투|GetUnitDirection))) -0.25) (>= (.X (Math|Vector|BreakVector (Variables|전투|GetUnitDirection))) -0.95)) (and (<= (.Y (Math|Vector|BreakVector (Variables|전투|GetUnitDirection))) -0.1) (>= (.Y (Math|Vector|BreakVector (Variables|전투|GetUnitDirection))) -0.9)))
        (Development|PrintString "Left Up" true true "(R=0.000000,G=1.000000,B=0.000000,A=1.000000)")
        (bind _output_get_3 (Variables|전투|SetEnumAttackType "NewEnumerator2"))
        (Variables|전투|SetAttackType (Math|Conversions|ToInteger(Byte) _output_get_3))
        (if (< (Math|Vector|GetPointDistancetoLine _returnvalue_7 (Variables|전투|GetMousePositionPressed) _output_get) (Class|KismetMathLibrary|GetPointDistancetoSegment _returnvalue_7 (Variables|전투|GetMousePositionPressed) _returnvalue_5)) :!label _label
          (if (< (Class|KismetMathLibrary|GetPointDistancetoSegment _returnvalue_7 (Variables|전투|GetMousePositionPressed) _returnvalue_5) 3e+02)
            (Development|PrintString "Attack Success" true true "(R=0.000000,G=0.000000,B=1.000000,A=1.000000)" :!label _label_2)
            (else
              (Development|PrintString "Attack Failed" true true "(R=1.000000,G=1.000000,B=0.000000,A=1.000000)" :!label _label_3)
              (bind _output_get_4 (Variables|전투|SetEnumAttackType "NewEnumerator8"))
              (Variables|전투|SetAttackType (Math|Conversions|ToInteger(Byte) _output_get_4))))
          (elif (< (Math|Vector|GetPointDistancetoLine _returnvalue_7 (Variables|전투|GetMousePositionPressed) _output_get) 3e+02)
            (goto _label_2)
            (else
              (goto _label_3))))
        (elif (and (and (<= (.X (Math|Vector|BreakVector (Variables|전투|GetUnitDirection))) -0.25) (>= (.X (Math|Vector|BreakVector (Variables|전투|GetUnitDirection))) -0.95)) (and (<= (.Y (Math|Vector|BreakVector (Variables|전투|GetUnitDirection))) 0.9) (>= (.Y (Math|Vector|BreakVector (Variables|전투|GetUnitDirection))) 0.1)))
          (Development|PrintString "Left Down" true true "(R=0.000000,G=1.000000,B=0.000000,A=1.000000)")
          (bind _output_get_5 (Variables|전투|SetEnumAttackType "NewEnumerator0"))
          (Variables|전투|SetAttackType (Math|Conversions|ToInteger(Byte) _output_get_5))
          (goto _label)
          (elif (and (and (<= (.X (Math|Vector|BreakVector (Variables|전투|GetUnitDirection))) 0.95) (>= (.X (Math|Vector|BreakVector (Variables|전투|GetUnitDirection))) 0.25)) (and (<= (.Y (Math|Vector|BreakVector (Variables|전투|GetUnitDirection))) -0.1) (>= (.Y (Math|Vector|BreakVector (Variables|전투|GetUnitDirection))) -0.9)))
            (Development|PrintString "Right Up" true true "(R=0.000000,G=1.000000,B=0.000000,A=1.000000)")
            (bind _output_get_6 (Variables|전투|SetEnumAttackType "NewEnumerator3"))
            (Variables|전투|SetAttackType (Math|Conversions|ToInteger(Byte) _output_get_6))
            (goto _label)
            (elif (and (and (<= (.X (Math|Vector|BreakVector (Variables|전투|GetUnitDirection))) 0.95) (>= (.X (Math|Vector|BreakVector (Variables|전투|GetUnitDirection))) 0.25)) (and (<= (.Y (Math|Vector|BreakVector (Variables|전투|GetUnitDirection))) 0.9) (>= (.Y (Math|Vector|BreakVector (Variables|전투|GetUnitDirection))) 0.1)))
              (Development|PrintString "Right Down" true true "(R=0.000000,G=1.000000,B=0.000000,A=1.000000)")
              (bind _output_get_7 (Variables|전투|SetEnumAttackType "NewEnumerator1"))
              (Variables|전투|SetAttackType (Math|Conversions|ToInteger(Byte) _output_get_7))
              (goto _label)
              (elif (and (<= (.X (Math|Vector|BreakVector (Variables|전투|GetUnitDirection))) -0.9501) (and (<= (.Y (Math|Vector|BreakVector (Variables|전투|GetUnitDirection))) 0.1) (>= (.Y (Math|Vector|BreakVector (Variables|전투|GetUnitDirection))) -0.1)))
                (Development|PrintString "Left" true true "(R=0.000000,G=1.000000,B=0.000000,A=1.000000)")
                (bind _output_get_8 (Variables|전투|SetEnumAttackType "NewEnumerator4"))
                (Variables|전투|SetAttackType (Math|Conversions|ToInteger(Byte) _output_get_8))
                (goto _label)
                (elif (and (>= (.X (Math|Vector|BreakVector (Variables|전투|GetUnitDirection))) 0.95) (and (<= (.Y (Math|Vector|BreakVector (Variables|전투|GetUnitDirection))) 0.2) (>= (.Y (Math|Vector|BreakVector (Variables|전투|GetUnitDirection))) -0.2)))
                  (Development|PrintString "Right" true true "(R=0.000000,G=1.000000,B=0.000000,A=1.000000)")
                  (bind _output_get_9 (Variables|전투|SetEnumAttackType "NewEnumerator5"))
                  (Variables|전투|SetAttackType (Math|Conversions|ToInteger(Byte) _output_get_9))
                  (goto _label)
                  (elif (and (and (<= (.X (Math|Vector|BreakVector (Variables|전투|GetUnitDirection))) 0.4) (>= (.X (Math|Vector|BreakVector (Variables|전투|GetUnitDirection))) -0.4)) (<= (.Y (Math|Vector|BreakVector (Variables|전투|GetUnitDirection))) -0.9))
                    (Development|PrintString "Up" true true "(R=0.000000,G=1.000000,B=0.000000,A=1.000000)")
                    (bind _output_get_10 (Variables|전투|SetEnumAttackType "NewEnumerator6"))
                    (Variables|전투|SetAttackType (Math|Conversions|ToInteger(Byte) _output_get_10))
                    (goto _label)
                    (elif (and (and (<= (.X (Math|Vector|BreakVector (Variables|전투|GetUnitDirection))) 0.4) (>= (.X (Math|Vector|BreakVector (Variables|전투|GetUnitDirection))) -0.4)) (>= (.Y (Math|Vector|BreakVector (Variables|전투|GetUnitDirection))) 0.9))
                      (Development|PrintString "Down" true true "(R=0.000000,G=1.000000,B=0.000000,A=1.000000)")
                      (bind _output_get_11 (Variables|전투|SetEnumAttackType "NewEnumerator7"))
                      (Variables|전투|SetAttackType (Math|Conversions|ToInteger(Byte) _output_get_11))
                      (goto _label)))))))))
      (else
        (Development|PrintString "공격의 길이가 짧음")))))

(fn ConstructionScript)

(fn NewFunction0
  (params (InVector2D :type Vector%202D%20Structure))
  (return (Math|Conversions|ToVector(Vector2D) InVector2D)))

(fn OnRepAvoidCoolTime)

(fn PauseGame
  (bind _returnvalue (Game|GetPlayerController 0))
  (Game|SetGamePaused true)
  (bind _returnvalue_2 (UserInterface|CreateWidget "/Game/BluePrint/PauseMenu.PauseMenu_C"))
  (bind _output_get (Variables|Default|SetPause%20Ref _returnvalue_2))
  (UserInterface|Viewport|AddtoViewport _output_get 0)
  (Variables|/Script/Engine.PlayerController|SetbShowMouseCursor _returnvalue true)
  (Input|SetInputModeUIOnly _returnvalue (Variables|Default|GetPause%20Ref) "LockAlways"))

(fn UnpauseGame
  (bind _returnvalue (Game|GetPlayerController 0))
  (Game|SetGamePaused false)
  (Widget|RemovefromParent (Variables|Default|GetPause%20Ref))
  (Input|SetInputModeGameOnly _returnvalue)
  (Variables|/Script/Engine.PlayerController|SetbShowMouseCursor _returnvalue false))