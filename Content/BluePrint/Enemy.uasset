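; Enemy Blueprint that tracks a monster's health and shows it on a health bar when an encounter starts.
; Any actor overlap casts the Name and HPWidget components' user widgets, then sets the bar to MaxHP and adds the health widget to the viewport.
; HP-- and HP++ events step HPMonster by one and refresh the stored widget's bar, with no clamping or death handling.
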(event Custom|HP--
  (bind _output_get (Variables|Default|SetHP%20Monster (- (Variables|Default|GetHP%20Monster) 1.0)))
  (Default|BarUpdate (stale Collision|EventActorBeginOverlap _asmonster_hp_widget) _output_get))

(event Custom|HP++
  (bind _output_get (Variables|Default|SetHP%20Monster (+ (Variables|Default|GetHP%20Monster) 1.0)))
  (Default|BarUpdate (stale Collision|EventActorBeginOverlap _asmonster_hp_widget) _output_get))

(event EventBeginPlay)

(event Collision|EventActorBeginOverlap
  (params (OtherActor :type Actor%20Object%20Reference))
  ;[1 1 1] 몬스터 체력(조우 했을때)
  (Utilities|Casting|CastToMonsterName (UserInterface|GetUserWidgetObject (Variables|Default|GetName)))
  (bind _asmonster_hp_widget (Utilities|Casting|CastToMonsterHP_Widget (UserInterface|GetUserWidgetObject (Variables|Default|GetHP_Widget))))
  (Default|BarUpdate _asmonster_hp_widget (Variables|Default|GetMaxHP))
  (UserInterface|Viewport|AddtoViewport _asmonster_hp_widget 0))

(event EventTick
  (params (DeltaSeconds :type Float%20%28single-precision%29)))

(fn ConstructionScript)