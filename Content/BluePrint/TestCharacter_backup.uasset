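; Test player character with camera-relative movement, a HUD, and debug keys that change HP, weapon, shield and armor values.
; Overlapping an "Enemy" actor locks input, then zero-delay loops turn the view and walk toward it until BattleMode starts.
; In BattleMode, Tick keeps the view interpolated onto the target.
; Right-mouse drags print their diagonal direction and "attack success" when passing near a hardcoded screen center; no damage is applied.
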(event OnComponentBeginOverlap(EnemyFinderCollision)
  (params (OverlappedComponent :type Primitive%20Component%20Object%20Reference) (OtherActor :type Actor%20Object%20Reference) (OtherComp :type Primitive%20Component%20Object%20Reference) (OtherBodyIndex :type Integer) (bFromSweep :type Boolean) (SweepResult :type Hit%20Result%20Structure%20%28by%20ref%29))
  (bind _returnvalue (Pawn|GetControlRotation :!class /Script/Engine.Pawn))
  ;[1 1 1] 몬스터와 가까워지면 사용자의 입력을 막고 시선을 몬스터 앞쪽으로 천천히 옮기는 루프
  (if (Actor|ActorHasTag OtherActor "Enemy")
    (Variables|Default|SetLockonTarget OtherActor)
    (Variables|Default|SetNotMoveTime true)
    (Utilities|FlowControl|Delay 0.0 :!label _label)
    (Pawn|SetControlRotation (Game|GetPlayerController 0) (Math|Interpolation|RInterpTo _returnvalue (Math|Rotator|FindLookatRotation (Transformation|GetWorldLocation (Variables|Default|GetCamera)) (+ (Transformation|GetActorLocation (Variables|Default|GetLockonTarget)) "100.000000, 0,200.000000")) (Variables|Default|GetDeltaTime) 2.0))
    (if (Math|Rotator|Equal(Rotator) _returnvalue (Math|Rotator|FindLookatRotation (Transformation|GetWorldLocation (Variables|Default|GetCamera)) (+ (Transformation|GetActorLocation (Variables|Default|GetLockonTarget)) "100.000000, 0,200.000000")) 2.0)
      ;[1 1 1] 몬스터 앞으로 캐릭터가 이동하는 루프
      (Utilities|FlowControl|Delay 0.0 :!label _label_2)
      (Pawn|Input|AddMovementInput (Math|Vector|GetForwardVector (Variables|Default|GetCamera)) 1.0 false)
      (if (Math|Vector|Equal(Vector) (+ (Transformation|GetActorLocation (Variables|Default|GetLockonTarget)) "100.000000, 0,200.000000") (Transformation|GetWorldLocation (Variables|Default|GetCamera)) 1e+02)
        (Variables|Default|SetBattleMode true)
        (else
          (goto _label_2)))
      (else
        (goto _label)))))

(event OnComponentEndOverlap(EnemyFinderCollision)
  (params (OverlappedComponent :type Primitive%20Component%20Object%20Reference) (OtherActor :type Actor%20Object%20Reference) (OtherComp :type Primitive%20Component%20Object%20Reference) (OtherBodyIndex :type Integer)))

(event EventBeginPlay
  (bind _returnvalue (UserInterface|CreateWidget "/Game/BluePrint/HUD.HUD_C"))
  (UserInterface|Viewport|AddtoViewport _returnvalue 0))

(event Collision|EventActorBeginOverlap
  (params (OtherActor :type Actor%20Object%20Reference)))

(event EventTick
  (params (DeltaSeconds :type Float%20%28single-precision%29))
  (bind _lockontarget (Variables|Default|GetLockonTarget))
  ;[1 1 1] 캐릭터가 몬스터와 콜리전 오버랩될때의 락온기능
  (Variables|Default|SetDeltaTime DeltaSeconds)
  (if (Variables|Default|GetBattleMode)
    (Utilities|IsValid _lockontarget
      (:Is%20Valid
        (Pawn|SetControlRotation (Game|GetPlayerController 0) (Math|Interpolation|RInterpTo (Pawn|GetControlRotation :!class /Script/Engine.Pawn) (Math|Rotator|FindLookatRotation (Transformation|GetWorldLocation (Variables|Default|GetCamera)) (+ (Transformation|GetActorLocation _lockontarget) "0, 0,200.000000")) (Variables|Default|GetDeltaTime) 5.0))
        (Variables|Default|SetBattleMode true)))))

(event Input|ActionEvents|InputActionJump
  (params (Key :type Key%20Structure))
  (:Pressed
    (if (not (Variables|Default|GetNotMoveTime))
      (Character|Jump))))

(event Input|AxisEvents|InputAxisForward
  (params (AxisValue :type Float%20%28single-precision%29))
  (if (not (Variables|Default|GetNotMoveTime))
    (Pawn|Input|AddMovementInput (Math|Vector|GetForwardVector (Variables|Default|GetCamera)) AxisValue false)))

(event Input|AxisEvents|InputAxisRight
  (params (AxisValue :type Float%20%28single-precision%29))
  (if (not (Variables|Default|GetNotMoveTime))
    (Pawn|Input|AddMovementInput (Math|Vector|GetRightVector (Variables|Default|GetCamera)) AxisValue false)))

(event Input|AxisEvents|InputAxisLookUp
  (params (AxisValue :type Float%20%28single-precision%29))
  (if (not (Variables|Default|GetNotMoveTime))
    (Pawn|Input|AddControllerPitchInput AxisValue)))

(event Input|AxisEvents|InputAxisLookRight
  (params (AxisValue :type Float%20%28single-precision%29))
  (if (not (Variables|Default|GetNotMoveTime))
    (Pawn|Input|AddControllerYawInput AxisValue)))

(event Input|KeyboardEvents|J
  (params (Key :type Key%20Structure))
  ;[1 1 1] 각종 상호작용 키 (임시인것도 있음)
  (:Pressed
    (bind _output_get (Variables|Default|SetWeapon (- (Variables|Default|GetWeapon) 3.0)))
    (Default|CallUpdateWeapon _output_get)))

(event Input|KeyboardEvents|F
  (params (Key :type Key%20Structure))
  ;[1 1 1] 각종 상호작용 키 (임시인것도 있음)
  (:Pressed
    (bind _output_get (Variables|Default|SetHP (- (Variables|Default|GetHP) 3.0)))
    (Default|CallUpdateHP _output_get)))

(event Input|KeyboardEvents|G
  (params (Key :type Key%20Structure))
  ;[1 1 1] 각종 상호작용 키 (임시인것도 있음)
  (:Pressed
    (bind _output_get (Variables|Default|SetHP (- (Variables|Default|GetHP) 35.0)))
    (Default|CallUpdateHP _output_get)))

(event Input|KeyboardEvents|K
  (params (Key :type Key%20Structure))
  ;[1 1 1] 각종 상호작용 키 (임시인것도 있음)
  (:Pressed
    (bind _output_get (Variables|Default|SetShield (- (Variables|Default|GetShield) 3.0)))
    (Default|CallUpdateShield _output_get)))

(event Input|KeyboardEvents|L
  (params (Key :type Key%20Structure))
  ;[1 1 1] 각종 상호작용 키 (임시인것도 있음)
  (:Pressed
    (bind _output_get (Variables|Default|SetArmor (- (Variables|Default|GetArmor) 3.0)))
    (Default|CallUpdateArmor _output_get)))

(event Input|KeyboardEvents|1
  (params (Key :type Key%20Structure))
  (bind _max_hp (Variables|Default|GetMax%20Hp))
  ;[1 1 1] 각종 상호작용 키 (임시인것도 있음)
  ;;[1 1 1] 체력회복
  (:Pressed
    (Variables|Default|SetPressed1 true)
    (if (> (+ (Variables|Default|GetHP) 2e+01) _max_hp)
      (bind _output_get (Variables|Default|SetHP _max_hp))
      (Default|CallUpdateHP _output_get)
      (Development|PrintString (Utilities|String|ToString(Float) _output_get))
      (else
        (bind _output_get_2 (Variables|Default|SetHP (+ (Variables|Default|GetHP) 2e+01)))
        (Default|CallUpdateHP _output_get_2)
        (Development|PrintString (Utilities|String|ToString(Float) _output_get_2)))))
  (:Released
    (Variables|Default|SetPressed1 false)))

(event Input|KeyboardEvents|2
  (params (Key :type Key%20Structure))
  ;[1 1 1] 각종 상호작용 키 (임시인것도 있음)
  (:Pressed
    (Variables|Default|SetPressed2 true))
  (:Released
    (Variables|Default|SetPressed2 false)))

(event Input|MouseEvents|RightMouseButton
  (params (Key :type Key%20Structure))
  (:Pressed
    (bind _returnvalue (Class|WidgetLayoutLibrary|GetMousePositiononViewport)))
  (:Released
    (bind _returnvalue_2 (Class|WidgetLayoutLibrary|GetMousePositiononViewport))
    (if (and (< (.X (Math|Vector|BreakVector (Math|Vector|GetUnitDirection(Vector) (Math|Conversions|ToVector(Vector2D) _returnvalue) (Math|Conversions|ToVector(Vector2D) _returnvalue_2)))) 0.0) (< (.Y (Math|Vector|BreakVector (Math|Vector|GetUnitDirection(Vector) (Math|Conversions|ToVector(Vector2D) _returnvalue) (Math|Conversions|ToVector(Vector2D) _returnvalue_2)))) 0.0))
      (Development|PrintString "Left Up")
      (elif (and (< (.X (Math|Vector|BreakVector (Math|Vector|GetUnitDirection(Vector) (Math|Conversions|ToVector(Vector2D) _returnvalue) (Math|Conversions|ToVector(Vector2D) _returnvalue_2)))) 0.0) (< 0.0 (.Y (Math|Vector|BreakVector (Math|Vector|GetUnitDirection(Vector) (Math|Conversions|ToVector(Vector2D) _returnvalue) (Math|Conversions|ToVector(Vector2D) _returnvalue_2))))))
        (Development|PrintString "Left Down")
        (elif (and (< 0.0 (.X (Math|Vector|BreakVector (Math|Vector|GetUnitDirection(Vector) (Math|Conversions|ToVector(Vector2D) _returnvalue) (Math|Conversions|ToVector(Vector2D) _returnvalue_2))))) (< (.Y (Math|Vector|BreakVector (Math|Vector|GetUnitDirection(Vector) (Math|Conversions|ToVector(Vector2D) _returnvalue) (Math|Conversions|ToVector(Vector2D) _returnvalue_2)))) 0.0))
          (Development|PrintString "Right Up")
          (elif (and (< 0.0 (.X (Math|Vector|BreakVector (Math|Vector|GetUnitDirection(Vector) (Math|Conversions|ToVector(Vector2D) _returnvalue) (Math|Conversions|ToVector(Vector2D) _returnvalue_2))))) (< 0.0 (.Y (Math|Vector|BreakVector (Math|Vector|GetUnitDirection(Vector) (Math|Conversions|ToVector(Vector2D) _returnvalue) (Math|Conversions|ToVector(Vector2D) _returnvalue_2))))))
            (Development|PrintString "Right Down")))))
    (if (< (Math|Vector|GetPointDistancetoLine "960.000000,540.000000, 0" (Math|Conversions|ToVector(Vector2D) _returnvalue) (Math|Vector|GetUnitDirection(Vector) (Math|Conversions|ToVector(Vector2D) _returnvalue) (Math|Conversions|ToVector(Vector2D) _returnvalue_2))) (Class|KismetMathLibrary|GetPointDistancetoSegment "960.000000,540.000000, 0" (Math|Conversions|ToVector(Vector2D) _returnvalue) (Math|Conversions|ToVector(Vector2D) _returnvalue_2)))
      (if (< (Class|KismetMathLibrary|GetPointDistancetoSegment "960.000000,540.000000, 0" (Math|Conversions|ToVector(Vector2D) _returnvalue) (Math|Conversions|ToVector(Vector2D) _returnvalue_2)) 2e+02)
        (Development|PrintString "attack success" :!label _label))
      (elif (< (Math|Vector|GetPointDistancetoLine "960.000000,540.000000, 0" (Math|Conversions|ToVector(Vector2D) _returnvalue) (Math|Vector|GetUnitDirection(Vector) (Math|Conversions|ToVector(Vector2D) _returnvalue) (Math|Conversions|ToVector(Vector2D) _returnvalue_2))) 2e+02)
        (goto _label)))))

(fn ConstructionScript)