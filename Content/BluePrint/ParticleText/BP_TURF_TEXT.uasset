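; BP_TURF_TEXT is a particle text effect actor that plays an animated reveal when TextMove fires.
; A timeline lerps the local Y of four particle systems, spreading them from a tight row to wider spacing.
; When the timeline finishes, four more particle systems become visible one after another with short delays.
; UpdateText is empty, and its looping timer and name-cycling text logic are disconnected.
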(event Custom|Update%20Text)

(event Custom|TextMove
  (bind _새_트랙_0 (Timeline|타임라인_0 PlayFromStart)
    (:Update
      (Transformation|SetRelativeLocation (Variables|Default|GetParticleSystem) (Math|Vector|MakeVector 0.0 (Math|Float|Lerp 1.2e+02 5.2e+02 _새_트랙_0) 0.0) false false)
      (Transformation|SetRelativeLocation (Variables|Default|GetParticleSystem1) (Math|Vector|MakeVector 0.0 (Math|Float|Lerp 7e+01 3.2e+02 _새_트랙_0) 0.0) false false)
      (Transformation|SetRelativeLocation (Variables|Default|GetParticleSystem2) (Math|Vector|MakeVector 0.0 (Math|Float|Lerp 2e+01 7e+01 _새_트랙_0) 0.0) false false)
      (Transformation|SetRelativeLocation (Variables|Default|GetParticleSystem3) (Math|Vector|MakeVector 0.0 (Math|Float|Lerp -3e+01 -2e+02 _새_트랙_0) 0.0) false false))
    (:Finished
      (Rendering|SetVisibility (Variables|Default|GetParticleSystem4) true false)
      (Utilities|FlowControl|Delay 0.5)
      (Rendering|SetVisibility (Variables|Default|GetParticleSystem5) true false)
      (Utilities|FlowControl|Delay 0.5)
      (Rendering|SetVisibility (Variables|Default|GetParticleSystem6) true false)
      (Utilities|FlowControl|Delay 0.5)
      (Rendering|SetVisibility (Variables|Default|GetParticleSystem7) true false))))

(event EventBeginPlay)

(fn ConstructionScript)