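; PlayerSkillSphere is a skill-orb actor that bobs in place and reacts to the player's sword.
; A timeline, restarted on finish from BeginPlay onward, lerps the Sphere's relative height in an endless loop; its rotation lerp is disconnected.
; Sphere1's end-overlap checks for the PlayerSwordCollision tag, casts the owner to TestCharacter, then switches on SkillType to spawn an emitter, without granting any skill.
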(event OnComponentBeginOverlap(Sphere1)
  (params (OverlappedComponent :type Primitive%20Component%20Object%20Reference) (OtherActor :type Actor%20Object%20Reference) (OtherComp :type Primitive%20Component%20Object%20Reference) (OtherBodyIndex :type Integer) (bFromSweep :type Boolean) (SweepResult :type Hit%20Result%20Structure%20%28by%20ref%29)))

(event OnComponentEndOverlap(Sphere1)
  (params (OverlappedComponent :type Primitive%20Component%20Object%20Reference) (OtherActor :type Actor%20Object%20Reference) (OtherComp :type Primitive%20Component%20Object%20Reference) (OtherBodyIndex :type Integer))
  (if (Components|ComponentHasTag OverlappedComponent "PlayerSwordCollision")
    (Variables|Default|SetTestCharacter (.AsTest%20Character (Utilities|Casting|CastToTestCharacter (Components|GetOwner OverlappedComponent))))
    (switch int (Variables|Default|GetSkillType)
      (:0
        (Effects|SpawnEmitteratLocation 0 "0, 0, 0"))
      (:1
        (Effects|SpawnEmitteratLocation 0 "0, 0, 0")))))

(event Custom|Moving%20Up%20Down
  ;[1 1 1] 위 아래로 반복 이동
  (bind (_direction _movement _rotation) (Timeline|UpDownTimeline PlayFromStart)
    (:Update
      (Transformation|SetRelativeLocation (Variables|Default|GetSphere) (Math|Vector|Lerp(Vector) "0, 0, 0" "0, 0,100.000000" _movement) false false))
    (:Finished
      (CallFunction|MovingUpDown))))

(event EventBeginPlay
  (CallFunction|MovingUpDown))

(event Collision|EventActorBeginOverlap
  (params (OtherActor :type Actor%20Object%20Reference)))

(event EventTick
  (params (DeltaSeconds :type Float%20%28single-precision%29)))

(fn ConstructionScript)