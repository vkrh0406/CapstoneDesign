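; A skill pickup sphere that grants the player a fire or ice skill when touched by the right-hand sword.
; A self-restarting timeline bobs the sphere up and down, while InitSkill sets a lava or ice material by type.
; When the tagged sword collision ends overlap, it plays the matching effect and sound, calls UseSkill on TestCharacter's right controller, resets SkillNowTime and destroys itself.
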(event OnComponentBeginOverlap(SphereCollision)
  (params (OverlappedComponent :type Primitive%20Component%20Object%20Reference) (OtherActor :type Actor%20Object%20Reference) (OtherComp :type Primitive%20Component%20Object%20Reference) (OtherBodyIndex :type Integer) (bFromSweep :type Boolean) (SweepResult :type Hit%20Result%20Structure%20%28by%20ref%29))
  ;[1 1 1] 플레이어의 검에 닿으면 파티클 보여준뒤 플레이어에게 스킬부여
)

(event OnComponentEndOverlap(SphereCollision)
  (params (OverlappedComponent :type Primitive%20Component%20Object%20Reference) (OtherActor :type Actor%20Object%20Reference) (OtherComp :type Primitive%20Component%20Object%20Reference) (OtherBodyIndex :type Integer))
  ;[1 1 1] 플레이어의 검에 닿으면 파티클 보여준뒤 플레이어에게 스킬부여
  (if (Components|ComponentHasTag OtherComp (Utilities|Array|Get(acopy) (Variables|/Script/Engine.ActorComponent|GetComponentTags (Variables|/Game/BluePrint/BP_MotionControllerRight.BP_MotionControllerRight_C|GetSwordCollision (Variables|/Game/BluePrint/TestCharacter.TestCharacter_C|GetRight%20Controller (Variables|Default|GetTestCharacter))))))
    (Development|PrintString "Skill On")
    (switch int (Variables|Default|GetSkillType)
      (:0
        (Effects|SpawnEmitteratLocation "/Game/InfinityBladeEffects/Effects/FX_Mobile/Impacts/P_Impact_Shield_Fire.P_Impact_Shield_Fire" (Transformation|GetWorldLocation (Variables|Default|GetSphere)))
        (Audio|PlaySoundatLocation "/Game/StarterContent/Audio/Fire01_Cue.Fire01_Cue" (Transformation|GetWorldLocation (Variables|Default|GetSphere)))
        (Rendering|SetVisibility (Variables|Default|GetSphere) false false))
      (:1
        (Effects|SpawnEmitteratLocation "/Game/InfinityBladeEffects/Effects/FX_Mobile/ICE/combat/P_Break_IceWall.P_Break_IceWall" (Transformation|GetWorldLocation (Variables|Default|GetSphere)))
        (Audio|PlaySoundatLocation "/Game/Audio/ice-cracking-01.ice-cracking-01" (Transformation|GetWorldLocation (Variables|Default|GetSphere)))
        (Rendering|SetVisibility (Variables|Default|GetSphere) false false)))
    (Default|UseSkill (Variables|/Game/BluePrint/TestCharacter.TestCharacter_C|GetRight%20Controller (Variables|Default|GetTestCharacter)) (Variables|Default|GetSkillType))
    (Variables|/Game/BluePrint/TestCharacter.TestCharacter_C|SetSkillNowTime (Variables|Default|GetTestCharacter) 0.0)
    (Actor|DestroyActor)))

(event Custom|Moving%20Up%20Down
  ;[1 1 1] 위 아래로 반복 이동
  (bind (_direction _movement _rotation) (Timeline|UpDownTimeline PlayFromStart)
    (:Update
      (Transformation|SetRelativeLocation (Variables|Default|GetSphere) (Math|Vector|Lerp(Vector) "0, 0, 0" "0, 0,50.000000" _movement) false false))
    (:Finished
      (CallFunction|MovingUpDown))))

(event EventBeginPlay
  (CallFunction|MovingUpDown)
  (Variables|Default|SetTestCharacter (.AsTest%20Character (Utilities|Casting|CastToTestCharacter (Game|GetPlayerCharacter 0)))))

(event Collision|EventActorBeginOverlap
  (params (OtherActor :type Actor%20Object%20Reference)))

(event EventTick
  (params (DeltaSeconds :type Float%20%28single-precision%29)))

(fn ConstructionScript)

(fn InitSkill
  (params (Skilltype :type Integer))
  (switch int Skilltype
    (:0
      (Rendering|Material|SetMaterial (Variables|Default|GetSphere) 0 "/Game/InfinityBladeEffects/Environments/Fire/Env_Fire_Magma/Materials/M_Lava_flows_trans.M_Lava_flows_trans"))
    (:1
      (Rendering|Material|SetMaterial (Variables|Default|GetSphere) 0 "/Game/InfinityBladeEffects/Effects/FX_Materials/Damage/M_CrackedGround_Ice_01_INST.M_CrackedGround_Ice_01_INST"))))