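; Skill pickup actor that grants the player a fire or ice skill when struck by the sword.
; InitSkill sets the skill type and matching sphere material.
; When a component tagged like the right controller's sword ends overlap, it plays that type's effect and sound, calls UseSkill, resets the player's skill timer and destroys itself.
; An up-down bobbing timeline exists but is never triggered or applied.
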(event OnComponentEndOverlap(Sphere1)
  (params (OverlappedComponent :type Primitive%20Component%20Object%20Reference) (OtherActor :type Actor%20Object%20Reference) (OtherComp :type Primitive%20Component%20Object%20Reference) (OtherBodyIndex :type Integer))
  ;[1 1 1] 플레이어의 검에 닿으면 파티클 보여준뒤 플레이어에게 스킬부여
  (if (Components|ComponentHasTag OtherComp (Utilities|Array|Get(acopy) (Variables|/Script/Engine.ActorComponent|GetComponentTags (Variables|/Game/BluePrint/BP_MotionControllerRight.BP_MotionControllerRight_C|GetSwordCollision (Variables|/Game/BluePrint/TestCharacter.TestCharacter_C|GetRight%20Controller (Variables|Default|GetTestCharacter))))))
    (Development|PrintString "Skill On")
    (switch int (Variables|Default|GetSkillType)
      (:0
        (Effects|SpawnEmitteratLocation "/Game/InfinityBladeEffects/Effects/FX_Mobile/Impacts/P_Impact_Shield_Fire.P_Impact_Shield_Fire" (Transformation|GetWorldLocation (Variables|Default|GetSphere)))
        (Audio|PlaySoundatLocation 0 (Transformation|GetWorldLocation (Variables|Default|GetSphere1)))
        (Rendering|SetVisibility (Variables|Default|GetSphere1) false false))
      (:1
        (Effects|SpawnEmitteratLocation "/Game/InfinityBladeEffects/Effects/FX_Mobile/ICE/combat/P_Break_IceWall.P_Break_IceWall" (Transformation|GetWorldLocation (Variables|Default|GetSphere1)))
        (Audio|PlaySoundatLocation "/Game/Audio/ice-cracking-01.ice-cracking-01" (Transformation|GetWorldLocation (Variables|Default|GetSphere1)))
        (Rendering|SetVisibility (Variables|Default|GetSphere1) false false)))
    (Default|UseSkill (Variables|/Game/BluePrint/TestCharacter.TestCharacter_C|GetRight%20Controller (Variables|Default|GetTestCharacter)) (Variables|Default|GetSkillType))
    (Variables|/Game/BluePrint/TestCharacter.TestCharacter_C|SetSkillNowTime (Variables|Default|GetTestCharacter) 0.0)
    (Actor|DestroyActor)))

(event Custom|Moving%20Up%20Down
  ;[1 1 1] 위 아래로 반복 이동
  (bind (_direction _movement _rotation) (Timeline|UpDownTimeline PlayFromStart)
    (:Finished
      (CallFunction|MovingUpDown))))

(event EventBeginPlay
  (Variables|Default|SetTestCharacter (.AsTest%20Character (Utilities|Casting|CastToTestCharacter (Game|GetPlayerCharacter 0)))))

(event Collision|EventActorBeginOverlap
  (params (OtherActor :type Actor%20Object%20Reference)))

(event EventTick
  (params (DeltaSeconds :type Float%20%28single-precision%29)))

(fn ConstructionScript)

(fn InitSkill
  (params (Skilltype :type Integer))
  (bind _sphere (Variables|Default|GetSphere))
  (switch int Skilltype
    (:0
      (Rendering|Material|SetMaterial _sphere 0 "/Game/InfinityBladeEffects/Effects/FX_Materials/Fire/M_JaggedRockFire_MeshEmit_Lit.M_JaggedRockFire_MeshEmit_Lit")
      (Variables|Default|SetSkillType 0))
    (:1
      (Rendering|Material|SetMaterial _sphere 0 "/Game/InfinityBladeEffects/Effects/FX_Materials/ICE/M_IceBlastBase.M_IceBlastBase")
      (Variables|Default|SetSkillType 1))))