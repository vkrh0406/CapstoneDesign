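; BP_MainMenuWidget is an actor that shows the main menu widget through a stereo layer, as used for VR display.
; On BeginPlay it moves the StereoLayer to the player pawn's transform, converted relative to the actor.
; Tick waits until the MainMenu render target is valid, then uses a DoOnce to assign it as the StereoLayer texture a single time.
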(event EventBeginPlay
  (Transformation|SetRelativeTransform (Variables|Default|GetStereoLayer) (Class|KismetMathLibrary|ConvertTransformtoRelative (Transformation|GetActorTransform (Game|Player|GetPlayerPawn 0)) (Transformation|GetActorTransform)) false false))

(event Collision|EventActorBeginOverlap
  (params (OtherActor :type Actor%20Object%20Reference)))

(event EventTick
  (params (DeltaSeconds :type Float%20%28single-precision%29))
  (bind _mainmenu (Variables|Default|GetMainMenu))
  (bind _returnvalue (Class|WidgetComponent|GetRenderTarget _mainmenu))
  (Utilities|IsValid _returnvalue
    (:Is%20Valid
      (Utilities|FlowControl|DoOnce false
        (:Completed
          (Class|StereoLayerComponent|SetTexture (Variables|Default|GetStereoLayer) _returnvalue))))))

(fn ConstructionScript)